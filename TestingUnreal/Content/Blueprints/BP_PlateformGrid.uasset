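; Platform grid actor that recolors its nine plane pieces when something overlaps its trigger box.
; BeginPlay gathers the planes into an array.
; Each overlap runs ApplyRandomStyle, which randomly picks all blue, all red, all yellow, or a mixed style where every piece gets its own random choice of those three materials.
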(event `self.ReceiveBeginPlay`
  (bind _plateformpieces (`self.PlateformPieces`))
  ;[1 1 1] Adding the 9 layouts into a array
  (`KismetArrayLibrary.Array_Add` _plateformpieces (`self.Plane`))
  (`KismetArrayLibrary.Array_Add` _plateformpieces (`self.Plane1`))
  (`KismetArrayLibrary.Array_Add` _plateformpieces (`self.Plane2`))
  (`KismetArrayLibrary.Array_Add` _plateformpieces (`self.Plane3`))
  (`KismetArrayLibrary.Array_Add` _plateformpieces (`self.Plane4`))
  (`KismetArrayLibrary.Array_Add` _plateformpieces (`self.Plane5`))
  (`KismetArrayLibrary.Array_Add` _plateformpieces (`self.Plane6`))
  (`KismetArrayLibrary.Array_Add` _plateformpieces (`self.Plane7`))
  (`KismetArrayLibrary.Array_Add` _plateformpieces (`self.Plane8`)))

(event `self.TriggerBox.OnComponentBeginOverlap`
  (params (OverlappedComponent :type "PrimitiveComponent Object Reference") (OtherActor :type "Actor Object Reference") (OtherComp :type "PrimitiveComponent Object Reference") (OtherBodyIndex :type Integer) (bFromSweep :type Boolean) (SweepResult :type "HitResult Structure (by ref)"))
  ;[1 1 1] Trigger
  (`KismetSystemLibrary.PrintString` "Trigger to change style")
  (`self.ApplyRandomStyle`))

(event `ApplyRandomStyle`
  ;[0.3594 0.3594 0.3594] ApplyRandomStyle
  (bind _output_get (set `self.RandomStyle` (`KismetMathLibrary.RandomIntegerInRange` 0 3)))
  (switch `int` _output_get
    (:`0`
      ;;[0.04803 0.6319 1] Blue
      (for _array_element (`self.PlateformPieces`)
        (`PrimitiveComponent.SetMaterial` _array_element 0 "/Game/Material/M_Blue.M_Blue")))
    (:`1`
      ;;[1 0.07955 0.1592] Red
      (for _array_element_2 (`self.PlateformPieces`)
        (`PrimitiveComponent.SetMaterial` _array_element_2 0 "/Game/Material/M_Red.M_Red")))
    (:`2`
      ;;[1 0.8306 0.1816] Yellow
      (for _array_element_3 (`self.PlateformPieces`)
        (`PrimitiveComponent.SetMaterial` _array_element_3 0 "/Game/Material/M_Yellow.M_Yellow")))
    (:`3`
      ;;[1 1 1] Random
      (for _array_element_4 (`self.PlateformPieces`)
        (`PrimitiveComponent.SetMaterial` _array_element_4 0 (select `int` (`KismetMathLibrary.RandomIntegerInRange` 0 2) :`0` "/Game/Material/M_Blue.M_Blue" :`1` "/Game/Material/M_Red.M_Red" :`2` "/Game/Material/M_Yellow.M_Yellow" :!type "MaterialInterface Object Reference"))))))

(fn `UserConstructionScript`)