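; BP_RoundManager runs an endless cycle of timed rounds that restyles a platform grid.
; StartRound, first called on BeginPlay, marks the round active, increments the round counter and, after a grid validity check, applies a random style to the grid and sets a timer.
; When the timer expires after RoundDuration, EndRound clears the active flag and immediately starts the next round.
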(event `self.ReceiveBeginPlay`
  (`self.StartRound`))

(event `StartRound`
  (`KismetSystemLibrary.PrintString` "RoundStart" true true (struct :`R` 0.032179 :`G` 1.0 :`B` 0.020612 :`A` 1.0))
  (set `self.RoundActive` true)
  (`/Engine/EditorBlueprintResources/StandardMacros.IncrementInt` (`self.CurrentRound`)
    (:`  `
      (`/Engine/EditorBlueprintResources/StandardMacros.IsValid` "/Game/Blueprints/BP_PlateformGrid.BP_PlateformGrid"
        (:`Is Valid`
          (`/Game/Blueprints/BP_PlateformGrid.ApplyRandomStyle` (`self.PlateFromGrid`))
          (bind _returnvalue (`KismetSystemLibrary.K2_SetTimer` null "EndRound" (`self.RoundDuration`)))
          (set `self.Timer` _returnvalue))))))

(event `EndRound`
  (set `self.RoundActive` false)
  (`KismetSystemLibrary.PrintString` "RoundEnd" true true (struct :`R` 1.0 :`G` 0.034709 :`A` 1.0))
  (`self.StartRound`))

(fn `UserConstructionScript`)